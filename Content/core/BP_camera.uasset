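; BP_camera is a camera pawn Blueprint that starts at a hardcoded, very distant world position.
; BeginPlay initializes its BPPawnMovement component, stores that position in OverallCamPos and calls init, which moves the collision component there without sweep and prints actual and target locations for debugging.
; Pressing J hides two specific building meshes, 101 and SmallHouse's Smallbuilding101, with no toggle to show them again.
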(event `self.ReceiveBeginPlay`
  ;[1 1 1] initialize
  (`/Game/core/BP_PawnMovement.InitComponent` (`self.BP_PawnMovement`))
  (set `self.overall_cam_pos` (-7000000.0 17500000.0 35000000.0))
  (`self.init`))

(event `init`
  (bind _collisioncomponent (`self.CollisionComponent`))
  (bind _overall_cam_pos (`self.overall_cam_pos`))
  (`SceneComponent.K2_SetWorldLocation` _collisioncomponent _overall_cam_pos false false)
  (`KismetSystemLibrary.PrintText` (`KismetTextLibrary.Conv_VectorToText` (`SceneComponent.K2_GetComponentLocation` _collisioncomponent)) true true (struct :`R` 0.645633 :`G` 0.178433 :`B` 1.0 :`A` 1.0))
  (`KismetSystemLibrary.PrintText` (`KismetTextLibrary.Conv_VectorToText` _overall_cam_pos) true true (struct :`R` 1.0 :`G` 0.051568 :`B` 0.081415 :`A` 1.0)))

(event `Key|J`
  (params (Key :type "Key Structure"))
  (:`Pressed`
    (`SceneComponent.SetVisibility` (`StaticMeshActor.StaticMeshComponent` (`self.101`)) false false)
    (`SceneComponent.SetVisibility` (`/Game/BuildingModels/AssetsStorage/BP_ToggleVisibility.smallbuilding101` (`self.SmallHouse`)) false false)))

(fn `UserConstructionScript`)