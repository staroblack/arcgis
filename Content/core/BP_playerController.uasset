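; Player controller Blueprint that toggles the screen between two UI widgets, UIPreprocessor and UIShowStatus.
; SwitchWidget flips the WhichOne boolean on each call, collapsing one widget and making the other visible.
; The event graph and construction script are empty, and the file shows neither widget creation nor a caller for the toggle.
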(fn `SwitchWidget`
  (if (`self.WhichOne`)
    (`Widget.SetVisibility` (`self.UIPreprocessor`) "Collapsed")
    (`Widget.SetVisibility` (`self.UIShowStatus`) "Visible")
    (set `self.WhichOne` false)
    (else
      (`Widget.SetVisibility` (`self.UIShowStatus`) "Collapsed")
      (`Widget.SetVisibility` (`self.UIPreprocessor`) "Visible")
      (set `self.WhichOne` true))))

(fn `UserConstructionScript`)