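; BP_moving pans the Camera actor across the horizontal plane while MiddlePushed is set, apparently for middle-mouse drag navigation.
; Each Tick turns the mouse delta since PreMousePosition into offsets along the camera's flattened forward and side vectors, then stores the new position.
; CanMouseMove selects a faster or slower pan speed.
; The camera's collision component moves without sweep, and neither flag is set in these graphs.
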(event `self.ReceiveTick`
  (params (DeltaSeconds :type "Float (single-precision)"))
  (bind (_pre_mouse_position_x _pre_mouse_position_y) (`KismetMathLibrary.BreakVector` (`self.Pre Mouse Position`)))
  (bind (_locationx _locationy) (`PlayerController.GetMousePosition` (`GameplayStatics.GetPlayerController` 0)))
  (bind _collisioncomponent (`DefaultPawn.CollisionComponent` (`self.camera`)))
  (bind (_returnvalue_x _returnvalue_y) (`KismetMathLibrary.BreakVector` (`SceneComponent.GetForwardVector` _collisioncomponent)))
  (bind (_returnvalue_x_2 _returnvalue_y_2) (`KismetMathLibrary.BreakVector` (`KismetMathLibrary.Cross_VectorVector` (`SceneComponent.GetForwardVector` _collisioncomponent) (0.0 0.0 1.0))))
  (bind _returnvalue (* (- _locationx _pre_mouse_position_x) (* (`self.speed`) -1.0)))
  (bind _returnvalue_2 (* (- _locationy _pre_mouse_position_y) (`self.speed`)))
  (if (`self.Middle Pushed`)
    (if (`self.can mouse move`)
      (set `self.speed` 20.0)
      (else
        (set `self.speed` 5.0)))
    (`SceneComponent.K2_SetWorldLocation` _collisioncomponent (+ (* (* (`KismetMathLibrary.Normal` (`KismetMathLibrary.MakeVector` _returnvalue_x_2 _returnvalue_y_2)) (`KismetMathLibrary.MakeVector` _returnvalue _returnvalue)) (-1.0 -1.0 0.0)) (+ (`SceneComponent.K2_GetComponentLocation` _collisioncomponent) (* (`KismetMathLibrary.Normal` (`KismetMathLibrary.MakeVector` _returnvalue_x _returnvalue_y)) (`KismetMathLibrary.MakeVector` _returnvalue_2 _returnvalue_2)))) false false)
    (set `self.Pre Mouse Position` (`KismetMathLibrary.MakeVector` _locationx _locationy))))

(fn `UserConstructionScript`)