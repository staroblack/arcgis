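; Movement component that pans its owning camera pawn across the world XY plane.
; On init it casts and caches the owner as the camera.
; BasicMovementControl turns two axis values, scaled by movement speed and a speed modifier, into world-space offsets on the camera's collision component, unless DisableCamera is set.
; Moves teleport-free and without sweep, and are not scaled by delta time.
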(event `InitComponent`
  (bind _ascamera (cast `/Game/core/camera` (`self.GetOwner`)))
  (set `self.As Camera` _ascamera))

(fn `BasicMovementControl`
  (params (`Axis Value X` :type "Float (double-precision)") (`Axis Value Y` :type "Float (double-precision)"))
  (locals (XLocal :type "Float (double-precision)") (YLocal :type "Float (double-precision)"))
  (bind _collisioncomponent (`DefaultPawn.CollisionComponent` (`self.As Camera`)))
  (bind _collisioncomponent_2 (`DefaultPawn.CollisionComponent` (`self.As Camera`)))
  (bind _collisioncomponent_3 (`DefaultPawn.CollisionComponent` (`self.As Camera`)))
  (set `local.XLocal` `Axis Value X`)
  (set `local.YLocal` `Axis Value Y`)
  (if (not (`self.bDisableCamera`))
    (if (and (!= (`local.XLocal`) 0.0) (!= (`local.YLocal`) 0.0))
      (`SceneComponent.K2_SetWorldLocation` _collisioncomponent_3 (+ (+ (`KismetMathLibrary.MakeVector` (* (`local.XLocal`) (`self.MovementSpeed`) (`self.SpeedModifier`))) (`KismetMathLibrary.MakeVector` 0.0 (* (`local.YLocal`) (`self.MovementSpeed`) (`self.SpeedModifier`)))) (`SceneComponent.K2_GetComponentLocation` _collisioncomponent_3)) false false)
      (elif (!= (`local.XLocal`) 0.0)
        (`SceneComponent.K2_SetWorldLocation` _collisioncomponent (+ (`SceneComponent.K2_GetComponentLocation` _collisioncomponent) (`KismetMathLibrary.MakeVector` (* (`local.XLocal`) (`self.MovementSpeed`) (`self.SpeedModifier`)))) false false)
        (elif (!= (`local.YLocal`) 0.0)
          (`SceneComponent.K2_SetWorldLocation` _collisioncomponent_2 (+ (`SceneComponent.K2_GetComponentLocation` _collisioncomponent_2) (`KismetMathLibrary.MakeVector` 0.0 (* (`local.YLocal`) (`self.MovementSpeed`) (`self.SpeedModifier`)))) false false))))))